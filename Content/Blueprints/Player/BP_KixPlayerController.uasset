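; Player controller for Kix that turns Enhanced Input look and move actions into view rotation and movement of the controlled pawn.
; BeginPlay registers the IMC_KixMovement mapping context and caches the pawn's movement component, though the move handler fetches it again.
; Look feeds yaw and pitch input directly.
; Move adds input vectors along the full control rotation's forward and right axes, so pitch affects the forward direction.
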(event `self.ReceiveBeginPlay`
  (`self.AddMappingContext`)
  (set `self.MovementComponent` (`Pawn.GetMovementComponent` (`self.K2_GetPawn`))))

(event `EnhancedInput|/Game/Blueprints/Input/Input_Actions/IA_Look`
  (params (ActionValue :type "Vector2D Structure") (ElapsedSeconds :type "Float (double-precision)") (TriggeredSeconds :type "Float (double-precision)") (InputAction :type "InputAction Object Reference" :default "/Game/Blueprints/Input/Input_Actions/IA_Look.IA_Look"))
  (:`Triggered`
    (`self.AddLookInput` ActionValue)))

(event `EnhancedInput|/Game/Blueprints/Input/Input_Actions/IA_Move`
  (params (ActionValue :type "Vector2D Structure") (ElapsedSeconds :type "Float (double-precision)") (TriggeredSeconds :type "Float (double-precision)") (InputAction :type "InputAction Object Reference" :default "/Game/Blueprints/Input/Input_Actions/IA_Move.IA_Move"))
  (bind _returnvalue_x (`KismetMathLibrary.BreakVector2D` (`|GetInputActionValue`)))
  (:`Triggered`
    (`PawnMovementComponent.AddInputVector` (`Pawn.GetMovementComponent` (`self.K2_GetPawn`)) (`self.GetForwardInput`) false)
    (`PawnMovementComponent.AddInputVector` (`Pawn.GetMovementComponent` (`self.K2_GetPawn`)) (* (`KismetMathLibrary.GetRightVector` (`self.GetControlRotation`)) _returnvalue_x) false)))

(fn `AddLookInput`
  (params (ActionValue :type "Vector2D Structure"))
  (bind (_x _y) (`KismetMathLibrary.BreakVector2D` ActionValue))
  (`self.AddYawInput` _x)
  (`self.AddPitchInput` _y))

(fn `AddMappingContext`
  (`EnhancedInputSubsystemInterface.AddMappingContext` (subsystem `EnhancedInputLocalPlayerSubsystem`) "/Game/Blueprints/Input/IMC_KixMovement.IMC_KixMovement" 0 (struct)))

(fn `GetForwardInput`
  (returns (ReturnValue :type "Vector Structure"))
  (bind (_returnvalue_x _returnvalue_y) (`KismetMathLibrary.BreakVector2D` (`|GetInputActionValue`)))
  (return (* (`KismetMathLibrary.GetForwardVector` (`self.GetControlRotation`)) _returnvalue_y)))

(fn `UserConstructionScript`)